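; BP_ShackerActor is a clickable shaker actor that feeds clicks into the game's BP_ClickManager.
; On BeginPlay it caches the first manager found, grants it BonusClicks and plays a one-shot skeletal mesh animation.
; Clicking its StaticMesh adds one click to that manager, without animating.
; OnShackerClicked replays the animation, but nothing in this Blueprint calls it.
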(event OnClicked(StaticMesh)
  (params (TouchedComponent :type Primitive%20Component%20Object%20Reference) (ButtonPressed :type Key%20Structure :default "None"))
  (Utilities|IsValid (Variables|Default|GetClickManagerRef)
    (:Is%20Valid
      (Default|AddClicks (Variables|Default|GetClickManagerRef) 1)
      (Development|PrintString "puntuando"))))

(event EventBeginPlay
  (bind _outactors (Actor|GetAllActorsOfClass "/Game/Blueprints/BP_ClickManager.BP_ClickManager_C"))
  (Utilities|IsValid (Utilities|Array|Get(acopy) _outactors)
    (:Is%20Valid
      (Variables|Default|SetClickManagerRef (Utilities|Array|Get(acopy) _outactors))
      (Default|AddClicks (Utilities|Array|Get(acopy) _outactors) (Variables|Default|GetBonusClicks))
      (Components|Animation|PlayAnimation (Variables|Default|GetSkeletalMesh) 0 false))
    (:Is%20Not%20Valid
      (Development|PrintString "Manager not found"))))

(event Collision|EventActorBeginOverlap
  (params (OtherActor :type Actor%20Object%20Reference)))

(fn ConstructionScript)

(fn OnShackerClicked
  (Components|Animation|PlayAnimation (Variables|Default|GetSkeletalMesh) 0 false))