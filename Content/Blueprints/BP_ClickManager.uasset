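; BP_ClickManager is an actor that tracks click and money totals for a click-driven game.
; AddClicks accumulates clicks and, whenever the nonzero total is an exact multiple of ClicksPerSpawn, spawns a SpawnClass actor at a hardcoded transform with a debug print.
; AddMoney only increases the Money balance, and BeginPlay calls AddClicks with zero, leaving the total unchanged.
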(event EventBeginPlay
  (CallFunction|AddClicks))

(event Collision|EventActorBeginOverlap
  (params (OtherActor :type Actor%20Object%20Reference)))

(event EventTick
  (params (DeltaSeconds :type Float%20%28single-precision%29)))

(fn ConstructionScript)

(fn AddClicks
  (params (Amount :type Integer))
  (Variables|Default|SetTotalClicks (+ Amount (Variables|Default|GetTotalClicks)))
  (if (!= (Variables|Default|GetTotalClicks) 0)
    (if (== (Math|Integer|%(Integer) (Variables|Default|GetTotalClicks) (Variables|Default|GetClicksPerSpawn)) 0)
      (bind _returnvalue (Game|SpawnActorfromClass (Variables|Default|GetSpawnClass) (Math|Transform|MakeTransform "1340.000000,6.000000,-210.000000") "AlwaysSpawn" "MultiplyWithRoot" 0 0))
      (Utilities|IsValid _returnvalue
        (:Is%20Valid
          (Development|PrintString "Spawn ok"))))))

(fn AddMoney
  (params (Amount :type Integer))
  (Variables|Default|SetMoney (+ (Variables|Default|GetMoney) Amount)))